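; BP_SetTest is a test Blueprint for Set container operations on VecSet.
; On BeginPlay it converts the set to an array twice, first looping by index and skipping the last two elements, then iterating every element, writing each visited value to Vec.
; Disconnected nodes lay out other set operations such as add, remove, clear, length and contains, but never execute.
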(event EventBeginPlay
  (Utilities|FlowControl|Sequence
    (:then_0
      (bind _result (Utilities|Set|ToArray (Variables|Default|GetVecSet)))
      (for _index (range 0 (Utilities|Array|LastIndex _result))
        (if (< _index (- (Utilities|Array|Length _result) 2))
          (Variables|Default|SetVec (Utilities|Array|Get(acopy) _result _index)))))
    (:then_1
      (bind _result_2 (Utilities|Set|ToArray (Variables|Default|GetVecSet)))
      (for _array_element _result_2
        (Variables|Default|SetVec _array_element)))))

(fn ConstructionScript)