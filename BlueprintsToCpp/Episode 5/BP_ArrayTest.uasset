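; BP_ArrayTest is a Blueprint sandbox that demonstrates operations on a vector array, with no gameplay effect.
; On BeginPlay it loops over VecArray by index, copying elements before the last two into Vec, then runs a for-each loop that copies every element into Vec.
; Unconnected nodes showcase other array functions such as add, insert, remove, append, clear, find and contains, but never execute.
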(event EventBeginPlay
  (bind _vecarray (Variables|Default|GetVecArray))
  (Utilities|FlowControl|Sequence
    (:then_0
      (for _index (range 0 (Utilities|Array|LastIndex _vecarray))
        (if (< _index (- (Utilities|Array|Length _vecarray) 2))
          (Variables|Default|SetVec (Utilities|Array|Get(acopy) _vecarray _index)))))
    (:then_1
      (for _array_element (Variables|Default|GetVecArray)
        (Variables|Default|SetVec _array_element)))))

(fn ConstructionScript)