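; BP_MapTest is a test Blueprint that exercises Map container operations on VecMap and ConeActorMap.
; BeginPlay loops over VecMap's keys and, for all but the last two indices, reads the value at key 0.
; InitializeConeActors fills ConeActorMap with every BP_Cone by index, then calls TestFunc on entry 0 if found.
; Unconnected nodes sample the other Map operations.
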(event Custom|InitializeConeActors
  (bind _coneactormap (Variables|Default|GetConeActorMap))
  (bind (_value _returnvalue) (Utilities|Map|Find _coneactormap 0))
  (Utilities|FlowControl|Sequence
    (:then_0
      (bind _outactors (Actor|GetAllActorsOfClass "/Game/Blueprints/BP_Cone.BP_Cone_C"))
      (for _index (range 0 (Utilities|Array|LastIndex _outactors))
        (Utilities|Map|Add (Variables|Default|GetConeActorMap) _index (Utilities|Array|Get(acopy) _outactors _index))))
    (:then_1
      (if _returnvalue
        (Class|ConeActor|TestFunc _value)))))

(event EventBeginPlay
  (bind _vecmap (Variables|Default|GetVecMap))
  (Utilities|FlowControl|Sequence
    (:then_0
      (bind _keys (Utilities|Map|Keys _vecmap))
      (for _index (range 0 (Utilities|Array|LastIndex _keys))
        (if (< _index (- (Utilities|Map|Length _vecmap) 2))
          (Variables|Default|SetVec (.Value (Utilities|Map|Find _vecmap 0))))))))

(fn ConstructionScript)